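; BP_IntimidationStatus is a battle status effect that halves the damage multiplier of the entity it targets.
; When applied, a DoOnce guard lets it store the target and its original multiplier and apply the reduction only once.
; When the effect ends, it prints a debug message and restores the stored multiplier.
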(event `self.DoStatusEffect`
  (params (entityTarget :type "BattleEntity Object Reference"))
  (`/Engine/EditorBlueprintResources/StandardMacros.DoOnce` false
    (:`Completed`
      (bind _output_get (set `self.EntityTarget` entityTarget))
      (bind _output_get_2 (set `self.OriginalDmgMultiplier` (`BattleEntity.DamageMultiplier` _output_get)))
      (set `BattleEntity.DamageMultiplier` (/ _output_get_2 2.0) (`self.EntityTarget`)))))

(event `self.OnEffectEnded`
  (`KismetSystemLibrary.PrintString` (`KismetStringLibrary.Concat_StrStr` (`self.StatusEffectName`) " has ended :C"))
  (set `BattleEntity.DamageMultiplier` (`self.OriginalDmgMultiplier`) (`self.EntityTarget`)))

(fn `UserConstructionScript`)