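; BP_TutorialTrap is a tutorial trap that sits on a battle grid cell.
; On activation it makes its parent cell explode with fixed damage and magnitude.
; Handlers to hide the mesh and to print a taunt and delete the cell exist, but the nodes binding them to trap-reset and cell-change events are disconnected, along with mesh-reveal and self-damage logic.
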(event `Hide Mesh`
  (`SceneComponent.SetHiddenInGame` (`self.MeshComponent`) true false))

(event `self.OnActivate`
  (params (entity :type "BattleEntity Object Reference"))
  (`BattleGridCell.Explode` (`self.ParentGridCell`) 2.0 1))

(event `Trap Triggered`
  (`KismetSystemLibrary.PrintString` "Aww, why you running away")
  (`BattleGridCell.DeleteCell` (`self.ParentGridCell`)))

(fn `UserConstructionScript`)