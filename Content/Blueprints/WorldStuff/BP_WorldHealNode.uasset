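; BP_WorldHealNode is a world node that restores the player's health to maximum the first time a unit arrives on it.
; It caches BP_DefaultInstance on BeginPlay and uses that game instance's VisitedCells list, keyed by actor location, to make the heal one-time.
; On arrival at an unvisited cell, it records the location and sets the instance's Health to MaxHealth.
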(event `self.ReceiveBeginPlay`
  (`parent.ReceiveBeginPlay`)
  (bind _asbp_default_instance (cast `/Game/Blueprints/BP_DefaultInstance` (`GameplayStatics.GetGameInstance`)))
  (set `self.DefaultInstance` _asbp_default_instance))

(event `self.OnUnitArrive`
  (bind _defaultinstance (`self.DefaultInstance`))
  (if (== (`KismetArrayLibrary.Array_Find` (`DefaultInstance.VisitedCells` (`self.DefaultInstance`)) (`self.K2_GetActorLocation`)) -1)
    (`KismetArrayLibrary.Array_AddUnique` (`DefaultInstance.VisitedCells` (`self.DefaultInstance`)) (`self.K2_GetActorLocation`))
    (set `DefaultInstance.Health` (`DefaultInstance.MaxHealth` _defaultinstance) _defaultinstance)))

(fn `UserConstructionScript`
  (`parent.UserConstructionScript`))