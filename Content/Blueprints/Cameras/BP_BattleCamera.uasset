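; Battle camera actor that frames the battle grid once at BeginPlay.
; InitialiseCamera averages the locations of all BattleGridCell actors to find the center and takes the square root of their count as grid size, implying a square grid.
; It moves the root to that center, pitches it by CameraAngle, offsets the camera backward in proportion to grid size, then aims it at the center.
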(event `self.ReceiveBeginPlay`
  (`self.InitialiseCamera`))

(fn `InitialiseCamera`
  (locals (CenterLocation :type "Vector Structure" :default (0.0 0.0 0.0)) (GridSize :type "Float (double-precision)" :default 0.0))
  (bind _defaultsceneroot (`self.DefaultSceneRoot`))
  (bind (_returnvalue_roll _returnvalue_pitch _returnvalue_yaw) (`KismetMathLibrary.BreakRotator` (`KismetMathLibrary.FindLookAtRotation` (`SceneComponent.K2_GetComponentLocation` (`self.Camera`)) (`local.CenterLocation`))))
  (bind _outactors (`GameplayStatics.GetAllActorsOfClass` "/Script/Terminal_Recall.BattleGridCell"))
  (bind _returnvalue (`GameplayStatics.GetActorArrayAverageLocation` _outactors))
  (set `local.CenterLocation` _returnvalue)
  (set `local.GridSize` (`KismetMathLibrary.Sqrt` (`KismetMathLibrary.Conv_IntToDouble` (`KismetArrayLibrary.Array_Length` _outactors))))
  (`SceneComponent.K2_SetWorldLocation` _defaultsceneroot (`local.CenterLocation`) false false)
  (`SceneComponent.K2_SetWorldRotation` _defaultsceneroot (`KismetMathLibrary.MakeRotator` 0.0 (`self.CameraAngle`)) false false)
  (`SceneComponent.K2_AddLocalOffset` (`self.Camera`) (`KismetMathLibrary.MakeVector` (* (`local.GridSize`) -125.0)) false false)
  (`SceneComponent.K2_SetWorldRotation` (`self.Camera`) (`KismetMathLibrary.MakeRotator` _returnvalue_roll _returnvalue_pitch _returnvalue_yaw) false false))

(fn `UserConstructionScript`)