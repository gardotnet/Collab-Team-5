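; Player-controlled camera actor that frames the world grid and supports WASD panning and mouse-wheel height adjustment.
; On construction and BeginPlay, SetInitRotation offsets the camera from the average location of all BP_BaseWorldGridCell actors and aims it at that point.
; Held keys run looping timers, cleared on release, that nudge the camera along world axes in fixed steps without Tick.
; Raw key events are marked for replacement with Enhanced Input.
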(event `self.ReceiveBeginPlay`
  (`self.SetInitRotation`))

(event `Key|A`
  (params (Key :type "Key Structure"))
  (:`Pressed`
    ; Replace with Triggered in Enhanced IA
    (bind _returnvalue (`KismetSystemLibrary.K2_SetTimerDelegate` (delegate `AddLeft`) 0.01 true)))
  (:`Released`
    (`KismetSystemLibrary.K2_ClearAndInvalidateTimerHandle` _returnvalue)))

(event `Key|W`
  (params (Key :type "Key Structure"))
  (:`Pressed`
    ; Replace with Triggered in Enhanced IA
    (bind _returnvalue (`KismetSystemLibrary.K2_SetTimerDelegate` (delegate `AddUp`) 0.01 true)))
  (:`Released`
    (`KismetSystemLibrary.K2_ClearAndInvalidateTimerHandle` _returnvalue)))

(event `AddLeft`
  (`SceneComponent.K2_AddWorldTransform` (`self.Camera`) (`KismetMathLibrary.MakeTransform` (0.0 -10.0 0.0)) false false))

(event `AddUp`
  (`SceneComponent.K2_AddWorldTransform` (`self.Camera`) (`KismetMathLibrary.MakeTransform` (10.0 0.0 0.0)) false false))

(event `Key|D`
  (params (Key :type "Key Structure"))
  (:`Pressed`
    ; Replace with Triggered in Enhanced IA
    (bind _returnvalue (`KismetSystemLibrary.K2_SetTimerDelegate` (delegate `AddRight`) 0.01 true)))
  (:`Released`
    (`KismetSystemLibrary.K2_ClearAndInvalidateTimerHandle` _returnvalue)))

(event `Key|S`
  (params (Key :type "Key Structure"))
  (:`Pressed`
    ; Replace with Triggered in Enhanced IA
    (bind _returnvalue (`KismetSystemLibrary.K2_SetTimerDelegate` (delegate `AddDown`) 0.01 true)))
  (:`Released`
    (`KismetSystemLibrary.K2_ClearAndInvalidateTimerHandle` _returnvalue)))

(event `AddRight`
  (`SceneComponent.K2_AddWorldTransform` (`self.Camera`) (`KismetMathLibrary.MakeTransform` (0.0 10.0 0.0)) false false))

(event `AddDown`
  (`SceneComponent.K2_AddWorldTransform` (`self.Camera`) (`KismetMathLibrary.MakeTransform` (-10.0 0.0 0.0)) false false))

(event `Key|MouseScrollUp`
  (params (Key :type "Key Structure"))
  (:`Pressed`
    (`SceneComponent.K2_AddWorldTransform` (`self.Camera`) (`KismetMathLibrary.MakeTransform` (0.0 0.0 -10.0)) false false)))

(event `Key|MouseScrollDown`
  (params (Key :type "Key Structure"))
  (:`Pressed`
    (`SceneComponent.K2_AddWorldTransform` (`self.Camera`) (`KismetMathLibrary.MakeTransform` (0.0 0.0 10.0)) false false)))

(fn `SetInitRotation`
  (bind _outactors (`GameplayStatics.GetAllActorsOfClass` "/Game/Blueprints/GridCells/BP_BaseWorldGridCell.BP_BaseWorldGridCell_C"))
  (bind _returnvalue (`GameplayStatics.GetActorArrayAverageLocation` _outactors))
  (`SceneComponent.K2_SetWorldLocation` (`self.Camera`) (+ _returnvalue (`KismetMathLibrary.MakeVector` (`self.CameraXOffset`) 0.0 (`self.CameraHeight`))) false false)
  (bind (_returnvalue_roll _returnvalue_pitch _returnvalue_yaw) (`KismetMathLibrary.BreakRotator` (`KismetMathLibrary.FindLookAtRotation` (`SceneComponent.K2_GetComponentLocation` (`self.Camera`)) _returnvalue)))
  (`SceneComponent.K2_SetWorldRotation` (`self.Camera`) (`KismetMathLibrary.MakeRotator` _returnvalue_roll _returnvalue_pitch _returnvalue_yaw) false false))

(fn `UserConstructionScript`
  (`self.SetInitRotation`))