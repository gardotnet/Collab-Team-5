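; BP_AutoCamera is a camera actor that automatically frames the BP_BaseWorldGridCell actors in the level.
; Its construction script calls SetTargetAverage, which offsets the camera from the cells' average location by the root's world X and Z, then aims it back at that point.
; SetTargetCurrentActive, uncalled here, does the same per cell, but its always-true condition leaves the camera on the last one.
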(fn `SetTargetAverage`
  (bind (_returnvalue_x _returnvalue_y _returnvalue_z) (`KismetMathLibrary.BreakVector` (`SceneComponent.K2_GetComponentLocation` (`self.DefaultSceneRoot`))))
  (bind _outactors (`GameplayStatics.GetAllActorsOfClass` "/Game/Blueprints/GridCells/BP_BaseWorldGridCell.BP_BaseWorldGridCell_C"))
  (bind _returnvalue (`GameplayStatics.GetActorArrayAverageLocation` _outactors))
  (`SceneComponent.K2_SetWorldLocation` (`self.Camera`) (+ _returnvalue (`KismetMathLibrary.MakeVector` _returnvalue_x 0.0 _returnvalue_z)) false false)
  (bind (_returnvalue_roll _returnvalue_pitch _returnvalue_yaw) (`KismetMathLibrary.BreakRotator` (`KismetMathLibrary.FindLookAtRotation` (`SceneComponent.K2_GetComponentLocation` (`self.Camera`)) _returnvalue)))
  (`SceneComponent.K2_SetWorldRotation` (`self.Camera`) (`KismetMathLibrary.MakeRotator` _returnvalue_roll _returnvalue_pitch _returnvalue_yaw) false false))

(fn `SetTargetCurrentActive`
  (bind (_returnvalue_x _returnvalue_y _returnvalue_z) (`KismetMathLibrary.BreakVector` (`SceneComponent.K2_GetComponentLocation` (`self.DefaultSceneRoot`))))
  (bind _outactors (`GameplayStatics.GetAllActorsOfClass` "/Game/Blueprints/GridCells/BP_BaseWorldGridCell.BP_BaseWorldGridCell_C"))
  (for _array_element _outactors
    (if true
      (bind _returnvalue (`SceneComponent.K2_GetComponentLocation` (`BaseGridCell.BoxComponent` _array_element)))
      (`SceneComponent.K2_SetWorldLocation` (`self.Camera`) (+ _returnvalue (`KismetMathLibrary.MakeVector` _returnvalue_x 0.0 _returnvalue_z)) false false)
      (bind (_returnvalue_roll _returnvalue_pitch _returnvalue_yaw) (`KismetMathLibrary.BreakRotator` (`KismetMathLibrary.FindLookAtRotation` (`SceneComponent.K2_GetComponentLocation` (`self.Camera`)) _returnvalue)))
      (`SceneComponent.K2_SetWorldRotation` (`self.Camera`) (`KismetMathLibrary.MakeRotator` _returnvalue_roll _returnvalue_pitch _returnvalue_yaw) false false))))

(fn `UserConstructionScript`
  (`self.SetTargetAverage`))