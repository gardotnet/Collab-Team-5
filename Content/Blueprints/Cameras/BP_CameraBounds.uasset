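; Placeable camera bounds actor that defines a rectangular area, presumably for limiting camera movement.
; The construction script sizes BoundBox from CameraBoxSize with a fixed, shallow vertical extent.
; It derives world-space X and Y edges from the box location plus and minus that size, but writes both sides to XPos and YPos, leaving only the minimum edges.
; The event graph has no active logic.
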(fn `UserConstructionScript`
  (bind (_cameraboxsize_x _cameraboxsize_y) (`KismetMathLibrary.BreakVector2D` (`self.CameraBoxSize`)))
  (bind (_cameraboxsize_x_2 _cameraboxsize_y_2) (`KismetMathLibrary.BreakVector2D` (`self.CameraBoxSize`)))
  (bind (_returnvalue_x _returnvalue_y) (`KismetMathLibrary.BreakVector` (`SceneComponent.K2_GetComponentLocation` (`self.BoundBox`))))
  (`BoxComponent.SetBoxExtent` (`self.BoundBox`) (`KismetMathLibrary.MakeVector` _cameraboxsize_x _cameraboxsize_y 30.0) true)
  (set `self.+XPos` (+ _returnvalue_x _cameraboxsize_x_2))
  (set `self.-XPos` (+ _returnvalue_x (* _cameraboxsize_x_2 -1.0)))
  (set `self.+YPos` (+ _returnvalue_y _cameraboxsize_y_2))
  (set `self.-YPos` (+ _returnvalue_y (* _cameraboxsize_y_2 -1.0))))