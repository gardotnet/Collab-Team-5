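; Visual debug cell, apparently for a weight map, that tints a cube by its gradient value.
; One tick after BeginPlay, it creates a dynamic instance of a semi-transparent material on the cube.
; The Color parameter runs from black to red using ChosenGradient over MaxGradient, amplified tenfold and clamped, so it saturates at a tenth of the maximum.
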(event `self.ReceiveBeginPlay`
  (`KismetSystemLibrary.DelayUntilNextTick`)
  (bind _returnvalue (`PrimitiveComponent.CreateDynamicMaterialInstance` (`self.Cube`) 0 "/Game/C++Testing/Semi-Transparent_Inst.Semi-Transparent_Inst" "None"))
  (`MaterialInstanceDynamic.SetVectorParameterValue` _returnvalue "Color" (`.SpecifiedColor` (break `SlateColor` (make `SlateColor` (make `LinearColor` (`KismetMathLibrary.FClamp` (* (/ (`KismetMathLibrary.Conv_IntToDouble` (`self.chosenGradient`)) (`KismetMathLibrary.Conv_IntToDouble` (`self.maxGradient`))) 10.0)) 0.0 0.0))))))

(fn `UserConstructionScript`)